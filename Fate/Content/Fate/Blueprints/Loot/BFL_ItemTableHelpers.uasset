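; Blueprint function library for loot that looks up item rows in a data table.
; GetRowFromItemID matches on the ItemID field, and GetRowFromItemName matches on the Name field.
; Both do a linear scan over every row name, fetching each row and returning the first match, rather than looking up by row name directly.
; Neither function has an explicit return for when no row matches.
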(fn `GetRowFromItemID`
  (params (`Item ID` :type "/Game/Fate/Blueprints/Loot/C_ItemID Object Reference"))
  (returns (`Item Entry` :type "/Game/Fate/Blueprints/Loot/S_ItemEntry Structure"))
  (locals (`Data Table` :type "DataTable Object Reference" :default "/Script/Engine.DataTable'/Game/Fate/Blueprints/Loot/DT_LootTable.DT_LootTable'"))
  (bind _outrownames (`DataTableFunctionLibrary.GetDataTableRowNames` (`local.Data Table`)))
  (for _array_element _outrownames
    (bind _returnvalue (`|GetDataTableRow` (`local.Data Table`) _array_element)
      (:`then`
        (if (== (`.ItemID_24_5F11F6B74A9E0B964D73FC90DB6644D2` (break `/Game/Fate/Blueprints/Loot/S_ItemEntry` _returnvalue)) `Item ID`)
          (return _returnvalue))))))

(fn `GetRowFromItemName`
  (params (`Item Name` :type Name))
  (returns (`Item Entry` :type "/Game/Fate/Blueprints/Loot/S_ItemEntry Structure"))
  (locals (`Data Table` :type "DataTable Object Reference" :default "/Script/Engine.DataTable'/Game/Fate/Blueprints/Loot/DT_LootTable.DT_LootTable'"))
  (bind _outrownames (`DataTableFunctionLibrary.GetDataTableRowNames` (`local.Data Table`)))
  (for _array_element _outrownames
    (bind _returnvalue (`|GetDataTableRow` (`local.Data Table`) _array_element)
      (:`then`
        (if (== (`.Name_17_859B2480456DF38278B8C78C3F1A6649` (break `/Game/Fate/Blueprints/Loot/S_ItemEntry` _returnvalue)) `Item Name`)
          (return _returnvalue))))))